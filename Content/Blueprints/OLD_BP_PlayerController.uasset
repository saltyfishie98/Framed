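; Player controller, prefixed OLD, that drives the player character with Enhanced Input movement along the world X axis and jumping.
; BeginPlay adds the IMC_Main mapping context, then IA_Move feeds movement input and IA_Jump starts and stops jumps.
; Tick casts the player character to BP_Hero and prints the viewport size as debug output, leaving the hero camera lookups unused.
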(event Input|EnhancedActionEvents|EnhancedInputActionIA_Move
  (params (ActionValue :type Float%20%28double-precision%29) (ElapsedSeconds :type Float%20%28double-precision%29) (TriggeredSeconds :type Float%20%28double-precision%29) (InputAction :type Input%20Action%20Object%20Reference :default "/Game/Defaults/Input/IA_Move.IA_Move"))
  (:Triggered
    (Pawn|Input|AddMovementInput (Game|GetPlayerCharacter 0) "1.000000,0.000000,0.000000" ActionValue false)))

(event Input|EnhancedActionEvents|EnhancedInputActionIA_Jump
  (params (ActionValue :type Boolean) (ElapsedSeconds :type Float%20%28double-precision%29) (TriggeredSeconds :type Float%20%28double-precision%29) (InputAction :type Input%20Action%20Object%20Reference :default "/Game/Defaults/Input/IA_Jump.IA_Jump"))
  (bind _returnvalue (Game|GetPlayerCharacter 0))
  (:Triggered
    (Character|Jump _returnvalue))
  (:Completed
    (Character|StopJumping _returnvalue)))

(event EventBeginPlay
  (Input|AddMappingContext (PlayerController|LocalPlayerSubsystems|GetEnhancedInputLocalPlayerSubsystem) "/Game/Defaults/Input/IMC_Main.IMC_Main" 0 "(bIgnoreAllPressedKeysUntilRelease=True,bForceImmediately=False)"))

(event EventTick
  (params (DeltaSeconds :type Float%20%28single-precision%29))
  (bind _asbp_hero (Utilities|Casting|CastToBP_Hero (Game|GetPlayerCharacter 0)))
  (Development|PrintString (Utilities|String|ToString(Vector2d) (Viewport|GetViewportSize))))

(fn ConstructionScript)